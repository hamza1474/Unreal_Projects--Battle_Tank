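; Tank pawn Blueprint that turns player input into tank driving, camera aiming and firing.
; On BeginPlay it hands the tracks to a movement component and the barrel and turret to an aiming component, which also handles Fire.
; Triggers set each track's throttle directly, while move axes send forward and turn intents to the movement component.
; Aim axes rotate an azimuth gimbal and spring arm, scaled by frame time.
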(event EventBeginPlay
  (Class|TankMovementComponent|Initialise (Variables|Default|GetTankMovement) (Variables|Default|GetLeftTrack) (Variables|Default|GetRightTrack))
  (Class|TankAimingComponent|Initialise (Variables|Default|GetTankAiming1) (Variables|Default|GetBarrel) (Variables|Default|GetTurret)))

(event Input|ActionEvents|InputActionFire
  (params (Key :type Key%20Structure :default "None"))
  ;[1 1 1] Aim Input Binding
  (:Pressed
    (Class|TankAimingComponent|Fire (Variables|Default|GetTankAiming1))))

(event Input|AxisEvents|InputAxisLeftTrigger
  (params (AxisValue :type Float%20%28single-precision%29))
  ;[1 1 1] Tank Movement Binding
  (Class|TankTrack|SetThrottle (Variables|Default|GetLeftTrack) AxisValue))

(event Input|AxisEvents|InputAxisRightTrigger
  (params (AxisValue :type Float%20%28single-precision%29))
  ;[1 1 1] Tank Movement Binding
  (Class|TankTrack|SetThrottle (Variables|Default|GetRightTrack) AxisValue))

(event Input|AxisEvents|InputAxisMoveAxisY
  (params (AxisValue :type Float%20%28single-precision%29))
  ;[1 1 1] Tank Movement Binding
  (Class|TankMovementComponent|IntendMoveForward (Variables|Default|GetTankMovement) AxisValue))

(event Input|AxisEvents|InputAxisAimElevation
  (params (AxisValue :type Float%20%28single-precision%29))
  ;[1 1 1] Aim Input Binding
  (Transformation|AddLocalRotation (Variables|Default|GetSpringArm) (Math|Rotator|MakeRotator 0.0 (* AxisValue (Utilities|Time|GetWorldDeltaSeconds) 1e+02) 0.0) false false))

(event Input|AxisEvents|InputAxisMoveAxisX
  (params (AxisValue :type Float%20%28single-precision%29))
  ;[1 1 1] Tank Movement Binding
  (Class|TankMovementComponent|IntendTurnRight (Variables|Default|GetTankMovement) AxisValue))

(event Input|AxisEvents|InputAxisAimAzimuth
  (params (AxisValue :type Float%20%28single-precision%29))
  ;[1 1 1] Aim Input Binding
  (Transformation|AddLocalRotation (Variables|Default|GetAzimuth%20Gimbal) (Math|Rotator|MakeRotator 0.0 0.0 (* AxisValue (Utilities|Time|GetWorldDeltaSeconds) 1e+02)) false false))

(fn ConstructionScript)